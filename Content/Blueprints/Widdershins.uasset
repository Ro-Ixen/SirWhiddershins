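; Widdershins is a player-controlled 2D flipbook character with side-scrolling movement along X and jumping.
; The MoveRight axis event moves it, flips control yaw to face travel direction, and runs death and animation updates.
; A small state function picks the idle, running or jumping flipbook from falling and velocity.
; Dropping to Z zero or below spawns and possesses a new Widdershins at the saved start transform, without destroying the old one.
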(event Custom|Update%20Animation
  ;[1 0.009271 0] Update Animation
  (bind _outflip (CallFunction|AnimationStateMachine (AI|Components|NavMovement|IsFalling (Variables|Character|GetCharacterMovement)) (> (Math|Vector|VectorLength (Transformation|GetVelocity)) 0.0)))
  (Sprite|SetFlipbook (Variables|Default|GetSprite) _outflip))

(event EventBeginPlay
  (Variables|Default|SetSpawn%20Transform (Transformation|GetActorTransform)))

(event EventActorBeginOverlap
  (params (OtherActor :type Actor%20Object%20Reference)))

(event EventTick
  (params (DeltaSeconds :type Float%20%28single-precision%29)))

(event Input|ActionEvents|InputActionJump
  ;[0.1597 1 0] Jumping
  (:Pressed
    (Character|Jump)))

(event Input|AxisEvents|InputAxisMoveRight
  (params (AxisValue :type Float%20%28single-precision%29))
  ;[0.07246 1 0.01613] Movement with Rotation
  (Pawn|Input|AddMovementInput "1.000000, 0, 0" AxisValue false)
  (CallFunction|CheckDeath)
  (CallFunction|UpdateAnimation)
  (Math|Float|CompareFloat AxisValue 0.0
    (:>
      (Pawn|SetControlRotation (Pawn|GetController) (Class|KismetMathLibrary|MakeRot 0.0 0.0 0.0)))
    (:<
      (Pawn|SetControlRotation (Pawn|GetController) (Class|KismetMathLibrary|MakeRot 0.0 1.8e+02 0.0)))))

(fn ConstructionScript)

(fn AnimationStateMachine
  (params (isFalling :type Boolean) (isMoving :type Boolean))
  (if isFalling
    (LocalVariables|SetAnimationState "NewEnumerator2")
    (elif isMoving
      (LocalVariables|SetAnimationState "NewEnumerator1")
      (else
        (LocalVariables|SetAnimationState "NewEnumerator0"))))
  (return (Utilities|Select :Index (LocalVariables|GetAnimationState) :NewEnumerator0 (Variables|Animations|GetIdle%20Flipbook) :NewEnumerator1 (Variables|Animations|GetRunning%20Flipbook) :NewEnumerator2 (Variables|Animations|GetJumping%20Flipbook))))

(fn CheckDeath
  (if (<= (.Z (Math|Vector|BreakVector (Transformation|GetActorLocation))) 0.0)
    (bind _returnvalue (Game|SpawnActorfromClass "Widdershins_C" (Variables|Default|GetSpawn%20Transform) false 0))
    (Pawn|Possess (Game|GetPlayerController 0) _returnvalue)))